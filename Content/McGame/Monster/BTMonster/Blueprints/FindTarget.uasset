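; FindTarget is a behavior tree node that acquires a target for a monster AI.
; On each AI tick without a valid TargetActor, it scans all GameCommonCharacter actors, skipping the controlled BTCharacter.
; The first one within Distance, by squared-length check, is stored in TargetActor and the Target blackboard key.
; It selects by iteration order rather than proximity, and keeps the target while it remains valid, regardless of range.
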(event EventReceiveTickAI
  (params (OwnerController :type AI%20Controller%20Object%20Reference) (ControlledPawn :type Pawn%20Object%20Reference) (DeltaSeconds :type Float%20%28single-precision%29))
  (if (not (Utilities|IsValid (Variables|Default|GetTargetActor)))
    (bind _asbtcharacter (Utilities|Casting|CastToBTCharacter ControlledPawn))
    (bind _outactors (Actor|GetAllActorsOfClass "/Script/MCGame.GameCommonCharacter"))
    (bind _array_element (Utilities|Array|ForEachLoopwithBreak _outactors :!label _label)
      (:LoopBody
        (if (!= _array_element _asbtcharacter)
          (if (<= (Math|Vector|VectorLengthSquared (- (Transformation|GetActorLocation _array_element) (Transformation|GetActorLocation _asbtcharacter))) (Math|Float|Square (Variables|Default|GetDistance)))
            (Variables|Default|SetTargetActor _array_element)
            (Class|BTFunctionLibrary|SetBlackboardValueasObject (Variables|Default|GetTarget) _array_element)
            (goto _label Break)))))))